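; Grid visual actor that draws a grid's tiles in a flat view and a toggleable tactical view.
; Two child BP_GridMeshInst actors hold the instances: flat walkable tiles at a ground offset, and type-colored tactical meshes Z-scaled relative to the lowest tile.
; Tile updates replace instances by index; tactical mode hides "NotTactical" actors.
; Tactical changes made while off, or a new lowest Z, defer a full rebuild until next enable.
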(event `self.ReceiveBeginPlay`
  (`self.SetActorTickEnabled` false))

(fn `DestroyGridVisual`
  (`|ExecutionSequence`
    (:`then_0`
      (bind _gridmeshinst (`self.GridMeshInst`)
        (:`then`
          (`/Game/Blueprints/Core/Grid/Utilities/BP_GridMeshInst.ClearInstances` _gridmeshinst))
        (:`else`)))
    (:`then_1`
      (bind _gridmeshinsttactical (`self.GridMeshInstTactical`)
        (:`then`
          (`/Game/Blueprints/Core/Grid/Utilities/BP_GridMeshInst.ClearInstances` _gridmeshinsttactical))
        (:`else`)))
    (:`then_2`
      (`self.SetGridLowestZ` 999999.0))))

(fn `InitializeGridVisual`
  (params (Grid :type "/Game/Blueprints/Core/Grid/BP_Grid Object Reference"))
  (bind (_meshsize _mesh _meshmaterial) (break `/Game/Blueprints/Core/Grid/GridShape/S_GridShapeData` (`/Game/Blueprints/Core/Grid/BP_Grid.GetCurrentShapeData` (`self.Grid`))))
  (bind (_meshsize_2 _mesh_2 _meshmaterial_2 _flatmesh _flatmaterial) (break `/Game/Blueprints/Core/Grid/GridShape/S_GridShapeData` (`/Game/Blueprints/Core/Grid/BP_Grid.GetCurrentShapeData` (`self.Grid`))))
  (set `self.Grid` Grid)
  (set `self.GridMeshInst` (cast `/Game/Blueprints/Core/Grid/Utilities/BP_GridMeshInst` (`ChildActorComponent.ChildActor` (`self.ChildActor_GridMeshInst`)) :!pure true))
  (set `self.GridMeshInstTactical` (cast `/Game/Blueprints/Core/Grid/Utilities/BP_GridMeshInst` (`ChildActorComponent.ChildActor` (`self.ChildActor_GridMeshInst_Tactical`)) :!pure true))
  (`/Game/Blueprints/Core/Grid/Utilities/BP_GridMeshInst.InitializeGridMeshInst` (`self.GridMeshInst`) _flatmesh _flatmaterial false "QueryOnly")
  (`/Game/Blueprints/Core/Grid/Utilities/BP_GridMeshInst.InitializeGridMeshInst` (`self.GridMeshInstTactical`) _mesh _meshmaterial true "QueryOnly")
  (`self.K2_SetActorLocation` (0.0 0.0 0.0)) ; Center grid in world
  (`self.SetOffsetFromGround` (`self.OffsetFromGround`))
  (`self.SetGridLowestZ` 999999.0)
  (`self.SetIsTactical` (`self.IsTactical`)))

(fn `SetGridLowestZ`
  (params (LowestZ :type "Float (double-precision)" :default 999999.0))
  (set `self.GridLowestZ` LowestZ)
  (set `self.NeedToReGenerateTacticalOnNextEnable` true))

(fn `SetIsTactical`
  (params (IsTactical :type Boolean))
  (set `self.IsTactical` IsTactical)
  (`SceneComponent.SetHiddenInGame` (`self.ChildActor_GridMeshInst_Tactical`) (not (`self.IsTactical`)) false)
  (bind _outactors (`GameplayStatics.GetAllActorsWithTag` "NotTactical"))
  (for _array_element _outactors
    (`self.SetActorHiddenInGame` _array_element (`self.IsTactical`)))
  (if (and (`self.IsTactical`) (`self.NeedToReGenerateTacticalOnNextEnable`))
    (set `self.NeedToReGenerateTacticalOnNextEnable` false)
    (bind _values (`BlueprintMapLibrary.Map_Values` (`/Game/Blueprints/Core/Grid/BP_Grid.GridTiles` (`self.Grid`))))
    (for _array_element_2 _values
      (`self.UpdateTileVisualTactical` _array_element_2))))

(fn `SetOffsetFromGround`
  (params (Offset :type "Float (double-precision)"))
  (set `self.OffsetFromGround` Offset)
  (`SceneComponent.K2_SetRelativeLocation` (`self.ChildActor_GridMeshInst`) (`KismetMathLibrary.MakeVector` 0.0 0.0 (`self.OffsetFromGround`)) false false))

(fn `UpdateTileVisual`
  (params (Data :type "/Game/Blueprints/Core/Grid/Utilities/S_TileData Structure"))
  (bind (_data_index _data_type _data_transform _data_states) (break `/Game/Blueprints/Core/Grid/Utilities/S_TileData` (`local.Data`)))
  (bind (_data_index_2 _data_type_2) (break `/Game/Blueprints/Core/Grid/Utilities/S_TileData` (`local.Data`)))
  (`|ExecutionSequence`
    (:`then_0`
      (bind _gridmeshinst (`self.GridMeshInst`)
        (:`then`
          (`/Game/Blueprints/Core/Grid/Utilities/BP_GridMeshInst.RemoveInstance` _gridmeshinst _data_index_2)
          (if (`/Game/Blueprints/Core/Grid/Utilities/BFL_TileData.IsTileTypeWalkable` _data_type_2)
            (`/Game/Blueprints/Core/Grid/Utilities/BP_GridMeshInst.AddInstance` (`self.GridMeshInst`) _data_index _data_type _data_transform _data_states)))
        (:`else`)))
    (:`then_1`
      (`self.UpdateTileVisualTactical` Data))))

(fn `UpdateTileVisualTactical`
  (params (Data :type "/Game/Blueprints/Core/Grid/Utilities/S_TileData Structure"))
  (bind (_data_index _data_type _data_transform) (break `/Game/Blueprints/Core/Grid/Utilities/S_TileData` (`local.Data`)))
  (bind (_data_index_2 _data_type_2 _data_transform_2 _data_states) (break `/Game/Blueprints/Core/Grid/Utilities/S_TileData` (`local.Data`)))
  (bind (_data_index_3 _data_type_3 _data_transform_3) (break `/Game/Blueprints/Core/Grid/Utilities/S_TileData` (`local.Data`)))
  (bind (_data_index_4 _data_type_4) (break `/Game/Blueprints/Core/Grid/Utilities/S_TileData` (`local.Data`)))
  (bind _z (.z (`.MeshSize_2_E7AC29074BEEA347CE22A7BEB8AE9311` (break `/Game/Blueprints/Core/Grid/GridShape/S_GridShapeData` (`/Game/Blueprints/Core/Grid/BP_Grid.GetCurrentShapeData` (`self.Grid`))))))
  (`|ExecutionSequence`
    (:`then_0`
      (if (< (.z (.location _data_transform_3)) (`self.GridLowestZ`))
        (`self.SetGridLowestZ` (.z (.location _data_transform_3)))))
    (:`then_1`
      (if (`self.IsTactical`)
        (bind _gridmeshinsttactical (`self.GridMeshInstTactical`)
          (:`then`
            (`/Game/Blueprints/Core/Grid/Utilities/BP_GridMeshInst.RemoveInstance` _gridmeshinsttactical _data_index_4)
            (if (`|EnumInequality` _data_type_4 "NewEnumerator0")
              (`/Game/Blueprints/Core/Grid/Utilities/BP_GridMeshInst.AddInstance` (`self.GridMeshInstTactical`) _data_index_2 _data_type_2 (`KismetMathLibrary.MakeTransform` (.location _data_transform_2) (struct) (`KismetMathLibrary.MakeVector` (.x (.scale _data_transform_2)) (.y (.scale _data_transform_2)) (/ (+ (- (.z (.location _data_transform)) (`self.GridLowestZ`)) _z) _z))) _data_states)))
          (:`else`))
        (else
          (set `self.NeedToReGenerateTacticalOnNextEnable` true))))))

(fn `UserConstructionScript`)