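; Player grid action that selects a tile, with a single tile selected at a time.
; ExcuteAction removes a state from the previously selected tile, then stores the new index and adds that state to it through the PlayerActions grid.
; Passing the already selected index toggles selection off by resetting it to a -999 sentinel.
; On Destroyed, it runs the action with that sentinel to clear the current selection.
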(event `self.ReceiveDestroyed`
  (`self.ExcuteAction` (make `IntPoint` -999 -999)))

(fn `ExcuteAction`
  (params (Index :type "IntPoint Structure"))
  (bind _playeractions (`self.PlayerActions`))
  (bind _playeractions_2 (`self.PlayerActions`))
  (`/Game/Blueprints/Core/Grid/BP_Grid.RemoveStateFromTile` (`/Game/Blueprints/Core/Player/BP_PlayerActions.Grid` _playeractions_2) (`/Game/Blueprints/Core/Player/BP_PlayerActions.SelectedTile` _playeractions_2) "NewEnumerator2")
  (if (!= (`/Game/Blueprints/Core/Player/BP_PlayerActions.SelectedTile` (`self.PlayerActions`)) (`local.Index`))
    (set `/Game/Blueprints/Core/Player/BP_PlayerActions.SelectedTile` (`local.Index`) (`self.PlayerActions`))
    (`/Game/Blueprints/Core/Grid/BP_Grid.AddStatesToTile` (`/Game/Blueprints/Core/Player/BP_PlayerActions.Grid` _playeractions) (`/Game/Blueprints/Core/Player/BP_PlayerActions.SelectedTile` _playeractions) "NewEnumerator2")
    (else
      (set `/Game/Blueprints/Core/Player/BP_PlayerActions.SelectedTile` (make `IntPoint` -999 -999) (`self.PlayerActions`)))))

(fn `UserConstructionScript`
  (`parent.UserConstructionScript`))