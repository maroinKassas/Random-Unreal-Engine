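; Player camera pawn with an orthographic camera that pans, rotates and zooms from input.
; Axis inputs shift a desired location along the actor's forward and right vectors and adjust a clamped desired ortho width, while left and right actions step the desired yaw.
; Tick eases location, rotation and ortho width toward those targets with interpolation, which are seeded from the current state on BeginPlay.
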(event `self.ReceiveBeginPlay`
  (set `self.Location_Desired` (`self.K2_GetActorLocation`))
  (set `self.Zoom_Desired` (`CameraComponent.OrthoWidth` (`self.Camera`)))
  (set `self.Rotation_Desired` (`self.K2_GetActorRotation`)))

(event `self.ReceiveTick`
  (params (DeltaSeconds :type "Float (single-precision)"))
  (bind _camera (`self.Camera`))
  (`CameraComponent.SetOrthoWidth` _camera (`KismetMathLibrary.FInterpTo` (`CameraComponent.OrthoWidth` _camera) (`self.Zoom_Desired`) (`GameplayStatics.GetWorldDeltaSeconds`) (`self.Zoom_Interp`)))
  (`self.K2_SetActorLocation` (`KismetMathLibrary.VInterpTo` (`self.K2_GetActorLocation`) (`self.Location_Desired`) (`GameplayStatics.GetWorldDeltaSeconds`) (`self.Location_Interp`)))
  (`self.K2_SetActorRotation` (`KismetMathLibrary.RInterpTo` (`self.K2_GetActorRotation`) (`self.Rotation_Desired`) (`GameplayStatics.GetWorldDeltaSeconds`) (`self.Rotation_Interp`))))

(event `InputAxis|InputAxis_Zoom`
  (params (AxisValue :type "Float (single-precision)"))
  (set `self.Zoom_Desired` (`KismetMathLibrary.FClamp` (+ (`self.Zoom_Desired`) (* AxisValue (`self.Zoom_Speed`))) (`self.Zoom_Min`) (`self.Zoom_Max`))))

(event `InputAxis|InputAxis_Forward`
  (params (AxisValue :type "Float (single-precision)"))
  (set `self.Location_Desired` (+ (`self.Location_Desired`) (* (`self.GetActorForwardVector`) (* AxisValue (`self.Location_Speed`))))))

(event `InputAxis|InputAxis_Right`
  (params (AxisValue :type "Float (single-precision)"))
  (set `self.Location_Desired` (+ (`self.Location_Desired`) (* (`self.GetActorRightVector`) (* AxisValue (`self.Location_Speed`))))))

(event `InputAction|InputAction_RotationRight`
  (params (Key :type "Key Structure"))
  (:`Pressed`
    (set `self.Rotation_Desired` (`KismetMathLibrary.ComposeRotators` (`self.Rotation_Desired`) (`KismetMathLibrary.MakeRotator` 0.0 0.0 (- 0.0 (`self.Rotation_Speed`)))))))

(event `InputAction|InputAction_RotationLeft`
  (params (Key :type "Key Structure"))
  (:`Pressed`
    (set `self.Rotation_Desired` (`KismetMathLibrary.ComposeRotators` (`self.Rotation_Desired`) (`KismetMathLibrary.MakeRotator` 0.0 0.0 (`self.Rotation_Speed`))))))

(fn `UserConstructionScript`)